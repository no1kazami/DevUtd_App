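; Game instance Blueprint for Bigtamin, holding Android storage-permission handling and loading of the FBM_SaveGame save.
; The permission-granted event loads the game slot, creating and saving it first if absent, then stores the object and flags success.
; The chain that checks or requests write permission and binds that event is disconnected, and Init is empty, so nothing here starts the load.
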(event `self.ReceiveInit`)

(event `Android_PermissionGranted`
  (params (Permissions :type "Array of String (by ref)") (GrantResults :type "Array of Boolean (by ref)"))
  (if (`|GetArrayItem` GrantResults)
    (bind _returnvalue (`GameplayStatics.DoesSaveGameExist` "FBM_GameSlot"))
    (if _returnvalue
      (bind _returnvalue_2 (`GameplayStatics.LoadGameFromSlot` "FBM_GameSlot" :!label _label))
      (bind _asfbm_save_game (cast `FBM_SaveGame` _returnvalue_2))
      (set `self.DevUtdSaveGame` _asfbm_save_game)
      (set `self.bIsPermissionSuccess` true)
      (else
        (bind _returnvalue_3 (`GameplayStatics.CreateSaveGameObject` "/Script/Bigtamin.FBM_SaveGame"))
        (bind _returnvalue_4 (`GameplayStatics.SaveGameToSlot` _returnvalue_3 "FBM_GameSlot"))
        (if _returnvalue_4
          (goto _label))))))